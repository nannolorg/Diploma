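; Interactable item actor in the inventory system that the first-person character can select when nearby.
; For the Weapon item type, BeginPlay loads ItemStats from the WeaponList data table using ItemIndex.
; The construction script does the same lookup but sets ItemName to empty text.
; Sphere overlaps set the character's SelectedObject to this actor and toggle NearInteractableObject; leaving does not clear SelectedObject.
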(event OnComponentBeginOverlap(Sphere)
  (params (OverlappedComponent :type Primitive%20Component%20Object%20Reference) (OtherActor :type Actor%20Object%20Reference) (OtherComp :type Primitive%20Component%20Object%20Reference) (OtherBodyIndex :type Integer) (bFromSweep :type Boolean) (SweepResult :type Hit%20Result%20Structure%20%28by%20ref%29))
  (bind _asfirst_person_character (Utilities|Casting|CastToFirstPersonCharacter OtherActor))
  (Variables|/Game/Blueprint/Character/FirstPersonCharacter.FirstPersonCharacter_C|SetSelectedObject _asfirst_person_character self)
  (Variables|/Game/Blueprint/Character/FirstPersonCharacter.FirstPersonCharacter_C|SetNearInteractableObject _asfirst_person_character true))

(event OnComponentEndOverlap(Sphere)
  (params (OverlappedComponent :type Primitive%20Component%20Object%20Reference) (OtherActor :type Actor%20Object%20Reference) (OtherComp :type Primitive%20Component%20Object%20Reference) (OtherBodyIndex :type Integer))
  (bind _asfirst_person_character (Utilities|Casting|CastToFirstPersonCharacter OtherActor))
  (Variables|/Game/Blueprint/Character/FirstPersonCharacter.FirstPersonCharacter_C|SetSelectedObject _asfirst_person_character self)
  (Variables|/Game/Blueprint/Character/FirstPersonCharacter.FirstPersonCharacter_C|SetNearInteractableObject _asfirst_person_character false))

(event EventBeginPlay
  (switch Utilities|FlowControl|Switch|SwitchonEnum_ItemTypes (Variables|Default|GetItemTypes)
    (:NewEnumerator0
      (bind _returnvalue (Utilities|GetDataTableRow "/Game/Blueprint/Inventory/WeaponList.WeaponList" (Utilities|Array|Get(acopy) (Variables|Default|GetWeapon) (Variables|Default|GetItemIndex)))
        (:then
          (Variables|Default|SetItemStats _returnvalue))))))

(event Collision|EventActorBeginOverlap
  (params (OtherActor :type Actor%20Object%20Reference)))

(event EventTick
  (params (DeltaSeconds :type Float%20%28single-precision%29)))

(fn ConstructionScript
  (switch Utilities|FlowControl|Switch|SwitchonEnum_ItemTypes (Variables|Default|GetItemTypes)
    (:NewEnumerator0
      (Utilities|GetDataTableRow "/Game/Blueprint/Inventory/WeaponList.WeaponList" (Utilities|Array|Get(acopy) (Variables|Default|GetWeapon) (Variables|Default|GetItemIndex))
        (:then
          (Rendering|Components|TextRender|SetText (Variables|Default|GetItemName) (Utilities|Text|ToText(String) "")))))))