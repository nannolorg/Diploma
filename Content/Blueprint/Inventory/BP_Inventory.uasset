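; Inventory Blueprint that adds picked items to an inventory screen, sorted into Weapon and Food boxes with stacked duplicates.
; AddToInventory checks per-type name lists, creating a W_Item widget for new names or incrementing the count on the existing child at the matching index.
; UpdateItemStats shows the selected item's weight on the HUD.
; DropItem removes collected-item and name entries, choosing the list by the last added item's type, without touching widgets.
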(event EventBeginPlay)

(event Collision|EventActorBeginOverlap
  (params (OtherActor :type Actor%20Object%20Reference)))

(event EventTick
  (params (DeltaSeconds :type Float%20%28single-precision%29)))

(fn ConstructionScript)

(fn AddtoInventory
  (params (InventoryScreen :type W%20Inventory%20HUD%20Object%20Reference) (Item%20to%20Add :type BP%20Interact%20Object%20Object%20Reference))
  (bind (_itemindex _isunique_) (Utilities|DoesItemNameAlreadyExist?))
  (Variables|Default|SetInventoryHUD InventoryScreen)
  (Variables|Default|SetItemAdded Item%20to%20Add)
  (Utilities|Array|Clear (Variables|Default|GetItemName))
  (Utilities|FlowControl|Sequence
    (:then_0
      ;[0.3002 0.4681 1] Sorting through the item type
      (switch Utilities|FlowControl|Switch|SwitchonEnum_ItemTypes (Variables|/Game/Blueprint/Inventory/BP_InteractObject.BP_InteractObject_C|GetItemTypes (Variables|Default|GetItemAdded))
        (:NewEnumerator0
          (Variables|Default|SetItemTypeBox (Variables|/Game/Blueprint/UI/W_InventoryHUD.W_InventoryHUD_C|GetWeaponBox InventoryScreen))
          (Variables|Default|SetItemName (Variables|Default|GetWeaponName)))
        (:NewEnumerator2
          (Variables|Default|SetItemTypeBox (Variables|/Game/Blueprint/UI/W_InventoryHUD.W_InventoryHUD_C|GetFoodBox InventoryScreen))
          (Variables|Default|SetItemName (Variables|Default|GetFoodName)))))
    (:then_1
      ;[1 1 1] Get the New item Name
      (Variables|Default|SetNewItemName (.itemname (Variables|/Game/Blueprint/Inventory/BP_InteractObject.BP_InteractObject_C|GetItemStats (Variables|Default|GetItemAdded))))
      ;[1 0 0] Is the Item a duplicate? or Unique?
      (if _isunique_
        (switch Utilities|FlowControl|Switch|SwitchonEnum_ItemTypes (Variables|/Game/Blueprint/Inventory/BP_InteractObject.BP_InteractObject_C|GetItemTypes (Variables|Default|GetItemAdded))
          (:NewEnumerator0
            (Utilities|Array|AddUnique (Variables|Default|GetWeaponName) (Variables|Default|GetNewItemName)))
          (:NewEnumerator2
            (Utilities|Array|AddUnique (Variables|Default|GetFoodName) (Variables|Default|GetNewItemName))))
        ;[1 1 1] Add Item Widget into Inventory Screen Widget
        (bind _returnvalue (UserInterface|CreateWidget "/Game/Blueprint/UI/W_Item.W_Item_C" (Game|GetPlayerController 0)))
        ;;[1 1 1] Reference
        (bind _output_get (Variables|Default|SetItemWidget _returnvalue))
        (Variables|/Game/Blueprint/UI/W_Item.W_Item_C|SetPlayerInventory _output_get self)
        (Widget|Panel|AddChild (Variables|Default|GetItemTypeBox) (Variables|Default|GetItemWidget))
        ;[1 1 1] Set Name and NumberCount of that item into the widget
        (Rendering|Components|TextRender|SetText (Variables|/Game/Blueprint/UI/W_Item.W_Item_C|GetItemNameTxt (Variables|Default|GetItemWidget)) (Utilities|Text|ToText(String) (Variables|Default|GetNewItemName)))
        (bind _result (Math|Integer|IncrementInt (Variables|/Game/Blueprint/UI/W_Item.W_Item_C|GetItemCount (Variables|Default|GetItemWidget)))
          (:%20%20
            (Rendering|Components|TextRender|SetText (Variables|/Game/Blueprint/UI/W_Item.W_Item_C|GetItemCountTxt (Variables|Default|GetItemWidget)) (Utilities|Text|ToText(Integer) _result))
            ;[1 1 1] Create a Reference in Item Widget
            (Variables|/Game/Blueprint/UI/W_Item.W_Item_C|SetInventoryItem (Variables|Default|GetItemWidget) (Variables|/Game/Blueprint/Inventory/BP_InteractObject.BP_InteractObject_C|GetItemStats (Variables|Default|GetItemAdded)))))
        (else
          (Variables|Default|SetDuplicateItemIndex _itemindex)
          ;[1 1 1] Increase the count of the duplicated item
          (bind _result_2 (Math|Integer|IncrementInt (Variables|/Game/Blueprint/UI/W_Item.W_Item_C|GetItemCount (.AsW%20Item (Utilities|Casting|CastToW_Item (Utilities|Array|Get(acopy) (Class|PanelWidget|GetAllChildren (Variables|Default|GetItemTypeBox)) (Variables|Default|GetDuplicateItemIndex))))))
            (:%20%20
              (Rendering|Components|TextRender|SetText (Variables|/Game/Blueprint/UI/W_Item.W_Item_C|GetItemCountTxt (.AsW%20Item (Utilities|Casting|CastToW_Item (Utilities|Array|Get(acopy) (Class|PanelWidget|GetAllChildren (Variables|Default|GetItemTypeBox)) (Variables|Default|GetDuplicateItemIndex))))) (Utilities|Text|ToText(Integer) _result_2)))))))))

(fn UpdateItemStats
  (params (SelectedItem :type Struct%20Inventory%20Structure))
  (bind _inventoryhud (Variables|Default|GetInventoryHUD))
  (Utilities|IsValid _inventoryhud
    (:Is%20Valid
      (Rendering|Components|TextRender|SetText (Variables|/Game/Blueprint/UI/W_InventoryHUD.W_InventoryHUD_C|GetWeightCount _inventoryhud) (Utilities|Text|ToText(Float) (.weight SelectedItem) "HalfToEven")))))

(fn DropItem
  (params (ItemToDrop :type Struct%20Inventory%20Structure))
  (bind _itemname (Utilities|Struct|BreakStruct_Inventory ItemToDrop))
  (Utilities|Array|RemoveItem (Variables|Default|GetCollectedItem) ItemToDrop)
  (switch Utilities|FlowControl|Switch|SwitchonEnum_ItemTypes (Variables|/Game/Blueprint/Inventory/BP_InteractObject.BP_InteractObject_C|GetItemTypes (Variables|Default|GetItemAdded))
    (:NewEnumerator0
      (Utilities|Array|RemoveItem (Variables|Default|GetWeaponName) _itemname))
    (:NewEnumerator2
      (Utilities|Array|RemoveItem (Variables|Default|GetFoodName) _itemname))))